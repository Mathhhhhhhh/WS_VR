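; BP_Luciole is a firefly (luciole) companion in VR that hovers near the player's camera with a sine bob and can be grabbed.
; Tick lerps it toward that spot when not held, and a gate detects each release.
; A release advances a non-wrapping color counter and plays a timeline that damps throw velocity while scaling follow speed.
; Tick also blends the MPC_Luciole color parameter toward the chosen color.
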(event `self.ReceiveBeginPlay`
  (bind _asvrpawn (cast `/Game/VRTemplate/Blueprints/VRPawn` (`GameplayStatics.GetPlayerPawn` 0)))
  (set `self.As VRPawn` _asvrpawn))

(event `self.ReceiveTick`
  (params (DeltaSeconds :type "Float (single-precision)"))
  (`|ExecutionSequence`
    (:`then_0`
      (`self.KeepInCamera` DeltaSeconds))
    (:`then_1`
      (if (`/Game/VRTemplate/Blueprints/GrabComponent.bIsHeld` (`self.GrabComponent`))
        (goto _label :!via `Open`)
        (else
          (`/Engine/EditorBlueprintResources/StandardMacros.Gate` true :!label _label
            (:`Exit`
              (`|ExecutionSequence`
                (:`then_0`
                  (set `self.Compteur` (+ (`self.Compteur`) 1))
                  (switch `int` (`self.Compteur`)
                    (:`0`
                      (set `self.TargetColor` (`KismetMathLibrary.Conv_ColorToLinearColor` (`KismetMathLibrary.Conv_LinearColorToColor` (struct :`R` 1.0 :`G` 1.0 :`B` 1.0 :`A` 1.0)))))
                    (:`1`
                      (set `self.TargetColor` (`KismetMathLibrary.Conv_ColorToLinearColor` (`KismetMathLibrary.Conv_LinearColorToColor` (struct :`R` 1.0 :`G` 0.916666 :`A` 1.0)))))
                    (:`2`
                      (set `self.TargetColor` (`KismetMathLibrary.Conv_ColorToLinearColor` (`KismetMathLibrary.Conv_LinearColorToColor` (struct :`G` 0.01411 :`B` 1.0 :`A` 1.0)))))
                    (:`3`
                      (set `self.TargetColor` (`KismetMathLibrary.Conv_ColorToLinearColor` (`KismetMathLibrary.Conv_LinearColorToColor` (struct :`R` 1.0 :`B` 0.007289 :`A` 1.0)))))))
                (:`then_1`
                  (bind (_direction _alpha) (`Timeline|Timeline` :!via `PlayFromStart`)
                    (:`Update`
                      (`PrimitiveComponent.SetPhysicsLinearVelocity` (`self.Sphere`) (`KismetMathLibrary.VLerp` (`/Game/VRTemplate/Blueprints/GrabComponent.AverageVelocity` (`self.GrabComponent`)) (0.0 0.0 0.0) _alpha) false "None")
                      (set `self.Alpha` (* _alpha 7.0)))))
                (:`then_2`
                  (goto _label :!via `Close`))))))))
    (:`then_2`
      (bind _returnvalue (`KismetMaterialLibrary.GetVectorParameterValue` "/Game/Game/Luciole/MPC_Luciole.MPC_Luciole" "Color"))
      (`KismetMaterialLibrary.SetVectorParameterValue` "/Game/Game/Luciole/MPC_Luciole.MPC_Luciole" "Color" (`KismetMathLibrary.LinearColorLerp` _returnvalue (`self.TargetColor`) (* DeltaSeconds 2.25))))))

(fn `KeepInCamera`
  (params (`Delta Seconds` :type "Float (double-precision)"))
  (bind _camera (`/Game/VRTemplate/Blueprints/VRPawn.Camera` (`self.As VRPawn`)))
  (if (not (`/Game/VRTemplate/Blueprints/GrabComponent.bIsHeld` (`self.GrabComponent`)))
    (`self.K2_SetActorLocation` (`KismetMathLibrary.VLerp` (`self.K2_GetActorLocation`) (+ (+ (+ (`SceneComponent.K2_GetComponentLocation` _camera) (* (`SceneComponent.GetForwardVector` _camera) (50.0 50.0 0.0))) (* (`SceneComponent.GetRightVector` _camera) 20.0)) (`KismetMathLibrary.MakeVector` 0.0 0.0 (* (`KismetMathLibrary.Sin` (* (`GameplayStatics.GetTimeSeconds`) 3.0)) 4.0))) (* `Delta Seconds` (`self.Alpha`))) false true)))

(fn `UserConstructionScript`)