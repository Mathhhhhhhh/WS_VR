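; BP_Guitare is a grabbable guitar prop that tracks what enters its box while held.
; Overlap begin caches the other component's child velocity calculator, and overlap end clears it.
; Disconnected logic would detect strumming as exact and average velocity opposing along the guitar's forward axis, driving a decaying music volume.
; That logic and the sound spawning never run, since BeginPlay and Tick are empty.
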(event `self.ReceiveBeginPlay`)

(event `self.ReceiveTick`
  (params (DeltaSeconds :type "Float (single-precision)")))

(event `self.BoxGuitare.OnComponentBeginOverlap`
  (params (OverlappedComponent :type "PrimitiveComponent Object Reference") (OtherActor :type "Actor Object Reference") (OtherComp :type "PrimitiveComponent Object Reference") (OtherBodyIndex :type Integer) (bFromSweep :type Boolean) (SweepResult :type "HitResult Structure (by ref)"))
  (if (`/Game/VRTemplate/Blueprints/GrabComponent.bIsHeld` (`self.GrabComponent`))
    (bind _asbpc_velocity_calculator (cast `/Game/Game/BLUEPRINTS/BPC/BPC_VelocityCalculator` (`SceneComponent.GetChildComponent` OtherComp 0)))
    (set `self.As BPC Velocity Calculator` _asbpc_velocity_calculator)))

(event `self.BoxGuitare.OnComponentEndOverlap`
  (params (OverlappedComponent :type "PrimitiveComponent Object Reference") (OtherActor :type "Actor Object Reference") (OtherComp :type "PrimitiveComponent Object Reference") (OtherBodyIndex :type Integer))
  (set `self.As BPC Velocity Calculator` null))

(fn `UserConstructionScript`)