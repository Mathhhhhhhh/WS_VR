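; BP_Yggdrasil drives the Yggdrasil tree's shift between base color and emissive look, based on the final swing's state.
; On BeginPlay it caches the BP_BalancoireFinal actor, then reads its CouleurYgg flag every Tick.
; The flag eases the Alpha scalar in the MPC_Ygg material parameter collection toward one or back toward zero using delta-time lerps, with the return running twice as fast.
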(event `self.ReceiveBeginPlay`
  (bind _returnvalue (`GameplayStatics.GetActorOfClass` "/Game/Game/BP/BP_BalancoireFinal.BP_BalancoireFinal_C"))
  (bind _output_get (set `self.BalancoireFinal` _returnvalue)))

(event `GoToEmissive`
  (params (A :type "Float (double-precision)"))
  (bind _returnvalue (`KismetMaterialLibrary.GetScalarParameterValue` "/Game/MPC_Ygg.MPC_Ygg" "Alpha"))
  (`KismetMaterialLibrary.SetScalarParameterValue` "/Game/MPC_Ygg.MPC_Ygg" "Alpha" (`KismetMathLibrary.Lerp` _returnvalue 1.0 (* A 1.25))))

(event `self.ReceiveTick`
  (params (DeltaSeconds :type "Float (single-precision)"))
  (if (`/Game/Game/BP/BP_BalancoireFinal.CouleurYgg?` (stale `self.ReceiveBeginPlay` _output_get))
    (`self.GoToEmissive` DeltaSeconds)
    (else
      (`self.goToBaseColor` DeltaSeconds))))

(event `goToBaseColor`
  (params (A :type "Float (double-precision)"))
  (bind _returnvalue (`KismetMaterialLibrary.GetScalarParameterValue` "/Game/MPC_Ygg.MPC_Ygg" "Alpha"))
  (`KismetMaterialLibrary.SetScalarParameterValue` "/Game/MPC_Ygg.MPC_Ygg" "Alpha" (`KismetMathLibrary.Lerp` _returnvalue 0.0 (* A 2.5))))

(fn `UserConstructionScript`)