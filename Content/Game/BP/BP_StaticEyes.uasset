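; VR eye actor that turns its sphere to face the player camera, with one eye in a ring visible at a time.
; Eyes register in GameMode.StaticEyes in Index order by polling each frame, and only Index 0 starts visible.
; An unnormalized camera-forward dot marks an eye seen when ahead.
; Once behind, it hides and polls until the next eye is out of view before revealing it.
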(event `self.ReceiveBeginPlay`
  (bind _asvrpawn (cast `/Game/VRTemplate/Blueprints/VRPawn` (`GameplayStatics.GetPlayerPawn` 0)))
  (set `self.Player` _asvrpawn)
  (bind _asvrgame_mode (cast `/Game/VRTemplate/Blueprints/VRGameMode` (`GameplayStatics.GetGameMode`)))
  (set `self.GameMode` _asvrgame_mode)
  (`|ExecutionSequence`
    (:`then_0`
      (if (== (`self.Index`) (`KismetArrayLibrary.Array_Length` (`/Game/VRTemplate/Blueprints/VRGameMode.StaticEyes` (`self.GameMode`)))) :!label _label
        (`KismetArrayLibrary.Array_Add` (`/Game/VRTemplate/Blueprints/VRGameMode.StaticEyes` (`self.GameMode`)) self)
        (else
          (`KismetSystemLibrary.Delay` 0.0)
          (goto _label))))
    (:`then_1`
      (`SceneComponent.SetHiddenInGame` (`self.Sphere1`) (!= (`self.Index`) 0) true))))

(event `self.ReceiveTick`
  (params (DeltaSeconds :type "Float (single-precision)"))
  (bind _staticeyes (`/Game/VRTemplate/Blueprints/VRGameMode.StaticEyes` (`self.GameMode`)))
  (bind _camera (`/Game/VRTemplate/Blueprints/VRPawn.Camera` (`self.Player`)))
  (bind _returnvalue (mod (+ (`self.Index`) 1) (`KismetArrayLibrary.Array_Length` _staticeyes)))
  (bind _output (`|GetArrayItem` _staticeyes _returnvalue))
  (`SceneComponent.K2_SetWorldRotation` (`self.Sphere1`) (`KismetMathLibrary.FindLookAtRotation` (`SceneComponent.K2_GetComponentLocation` (`self.Sphere1`)) (`SceneComponent.K2_GetComponentLocation` (`/Game/VRTemplate/Blueprints/VRPawn.Camera` (`self.Player`)))) false false)
  (set `self.LazyFix` (`KismetMathLibrary.Dot_VectorVector` (`SceneComponent.GetForwardVector` _camera) (- (`self.K2_GetActorLocation`) (`SceneComponent.K2_GetComponentLocation` _camera))))
  (if (> (`self.LazyFix`) 0.35)
    (if (not (`SceneComponent.bHiddenInGame` (`self.Sphere1`)))
      (set `self.IsSeen` true)
      (`KismetSystemLibrary.PrintString` (`KismetStringLibrary.Concat_StrStr` (`KismetStringLibrary.Conv_IntToString` (`self.Index`)) "Seen")))
    (elif (and (`self.IsSeen`) (not (`SceneComponent.bHiddenInGame` (`self.Sphere1`))) (< (`self.LazyFix`) 0.0))
      (`SceneComponent.SetHiddenInGame` (`self.Sphere1`) true true)
      (if (< (`/Game/Game/BP/BP_StaticEyes.LazyFix` _output) 0.35) :!label _label_2
        (`SceneComponent.SetHiddenInGame` (`/Game/Game/BP/BP_StaticEyes.Sphere1` _output) false true)
        (set `/Game/Game/BP/BP_StaticEyes.IsSeen` false _output)
        (`KismetSystemLibrary.PrintString` (`KismetStringLibrary.Concat_StrStr` (`KismetStringLibrary.Conv_IntToString` _returnvalue) "Spawn"))
        (else
          (`KismetSystemLibrary.Delay` 0.0)
          (goto _label_2))))))

(fn `UserConstructionScript`
  (`SceneComponent.K2_SetWorldRotation` (`self.Sphere1`) (`KismetMathLibrary.MakeRotFromXZ` (`KismetMathLibrary.NegateVector` (`KismetMathLibrary.Normal` (`KismetMathLibrary.ProjectVectorOnToPlane` (`self.K2_GetActorLocation`) (0.0 0.0 1.0)))) (0.0 0.0 1.0)) false false))