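; BP_Branche is a branch actor that shrinks away and removes itself once it is flagged as destroyed.
; While IsDestroyed is set, Tick lerps the Cylinder component's relative scale toward zero at a frame-time-scaled rate, giving an eased shrink.
; When the scale vector becomes nearly zero, the actor destroys itself.
; Nothing in this graph sets the flag.
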(event `self.ReceiveBeginPlay`)

(event `self.ReceiveTick`
  (params (DeltaSeconds :type "Float (single-precision)"))
  (bind _cylinder (`self.Cylinder`))
  (bind _relativescale3d (`SceneComponent.RelativeScale3D` _cylinder))
  (if (`self.IsDestroyed`)
    (`SceneComponent.SetRelativeScale3D` _cylinder (`KismetMathLibrary.VLerp` _relativescale3d (0.0 0.0 0.0) (* DeltaSeconds 5.0)))
    (if (< (`KismetMathLibrary.VSize` _relativescale3d) 0.01)
      (`self.K2_DestroyActor`))))

(fn `UserConstructionScript`)