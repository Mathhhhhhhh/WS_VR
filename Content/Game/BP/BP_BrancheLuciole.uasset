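; BP_BrancheLuciole is a branch actor that attaches itself to Flar by following it once touched.
; When BP_Flar overlaps its capsule, it stores that reference and sets a follow flag, which this graph never clears.
; Each Tick while following, it zeroes the cylinder's physics velocity and teleports toward a point just below Flar, using a delta-time-scaled lerp for smooth trailing.
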(event `self.Capsule.OnComponentBeginOverlap`
  (params (OverlappedComponent :type "PrimitiveComponent Object Reference") (OtherActor :type "Actor Object Reference") (OtherComp :type "PrimitiveComponent Object Reference") (OtherBodyIndex :type Integer) (bFromSweep :type Boolean) (SweepResult :type "HitResult Structure (by ref)"))
  ;[1 0.3958 0.3958] Quand flar rentre dans la box de la branche elle active une bool pour l'event tick
  (bind _asbp_flar (cast `/Game/Game/Flar/BP_Flar` OtherActor))
  (set `self.Flar` _asbp_flar)
  (set `self.followflar` true))

(event `self.ReceiveTick`
  (params (DeltaSeconds :type "Float (single-precision)"))
  ;[1 1 1] Si la bool est activée la branche suit flar
  (`parent.ReceiveTick` DeltaSeconds)
  (if (`self.followflar`)
    (`PrimitiveComponent.SetPhysicsLinearVelocity` (`self.Cylinder`) (0.0 0.0 0.0) false "None")
    (`self.K2_SetActorLocation` (`KismetMathLibrary.VLerp` (`self.K2_GetActorLocation`) (+ (`self.K2_GetActorLocation` (`self.Flar`)) (0.0 0.0 -20.0)) (* DeltaSeconds 10.0)) false true)))

(fn `UserConstructionScript`
  (`parent.UserConstructionScript`))