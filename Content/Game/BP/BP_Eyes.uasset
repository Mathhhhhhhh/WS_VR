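; BP_Eyes is an actor whose eye sphere always faces the VR player's camera and flees when the player turns toward it.
; A per-tick, unnormalized dot product against camera forward triggers a timeline that slides Sphere1 along a spline with power easing.
; Turning away teleports the sphere back to its relative origin.
; The construction script yaws the spline and sphere toward the world origin.
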(event `self.ReceiveBeginPlay`
  (bind _asvrpawn (cast `/Game/VRTemplate/Blueprints/VRPawn` (`GameplayStatics.GetPlayerPawn` 0)))
  (set `self.Player` _asvrpawn))

(event `self.ReceiveTick`
  (params (DeltaSeconds :type "Float (single-precision)"))
  (bind _spline (`self.Spline`))
  (bind _camera (`/Game/VRTemplate/Blueprints/VRPawn.Camera` (`self.Player`)))
  (`SceneComponent.K2_SetWorldRotation` (`self.Sphere1`) (`KismetMathLibrary.FindLookAtRotation` (`SceneComponent.K2_GetComponentLocation` (`self.Sphere1`)) (`SceneComponent.K2_GetComponentLocation` (`/Game/VRTemplate/Blueprints/VRPawn.Camera` (`self.Player`)))) false false)
  (if (> (`KismetMathLibrary.Dot_VectorVector` (`SceneComponent.GetForwardVector` _camera) (- (`self.K2_GetActorLocation`) (`SceneComponent.K2_GetComponentLocation` _camera))) 0.35)
    (if (`self.IsVisible`)
      (set `self.IsVisible` false)
      (bind (_direction _alpha) (`Timeline|Timeline` :!via `PlayFromStart`)
        (:`Update`
          (`SceneComponent.K2_SetWorldLocation` (`self.Sphere1`) (`SplineComponent.GetLocationAtDistanceAlongSpline` _spline (* (`SplineComponent.GetSplineLength` _spline) (`KismetMathLibrary.MultiplyMultiply_FloatFloat` _alpha 2.5)) "World") false false))))
    (elif (not (`self.IsVisible`))
      (set `self.IsVisible` true)
      (`SceneComponent.K2_SetRelativeLocation` (`self.Sphere1`) (0.0 0.0 0.0) false true))))

(fn `UserConstructionScript`
  (`SceneComponent.K2_SetWorldRotation` (`self.Spline`) (`KismetMathLibrary.MakeRotFromXZ` (`KismetMathLibrary.NegateVector` (`KismetMathLibrary.Normal` (`KismetMathLibrary.ProjectVectorOnToPlane` (`self.K2_GetActorLocation`) (0.0 0.0 1.0)))) (0.0 0.0 1.0)) false false)
  (`SceneComponent.K2_SetWorldRotation` (`self.Sphere1`) (`KismetMathLibrary.MakeRotFromXZ` (`KismetMathLibrary.NegateVector` (`KismetMathLibrary.Normal` (`KismetMathLibrary.ProjectVectorOnToPlane` (`self.K2_GetActorLocation`) (0.0 0.0 1.0)))) (0.0 0.0 1.0)) false false))