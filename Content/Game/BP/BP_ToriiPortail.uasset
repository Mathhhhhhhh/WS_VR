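; BP_ToriiPortail is a torii portal that animates open and then acts as a level exit to ForestMap.
; One second after BeginPlay, the Portal timeline scales the Plane and shifts the level's BP_Sphere in Z, adding its Position track to the current height each update.
; When the timeline finishes, it creates the BPW_FonduFin widget without displaying it and sets IsEnd, which lets any Box overlap load ForestMap.
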(event `self.ReceiveBeginPlay`
  (bind _sphere (`self.Sphere`))
  (bind (_returnvalue_x _returnvalue_y _returnvalue_z) (`KismetMathLibrary.BreakVector` (`self.K2_GetActorLocation` _sphere)))
  (bind _returnvalue (`GameplayStatics.GetActorOfClass` "/Game/Game/FX/FX_Portal/FX_Portal/BP_Sphere.BP_Sphere_C"))
  (set `self.Sphere` _returnvalue)
  (`KismetSystemLibrary.Delay` 1.0)
  (bind (_direction _scale _position) (`Timeline|Portal` :!via `PlayFromStart`)
    (:`Update`
      (`SceneComponent.SetWorldScale3D` (`self.Plane`) (`KismetMathLibrary.Conv_DoubleToVector` _scale))
      (`self.K2_SetActorLocation` _sphere (`KismetMathLibrary.MakeVector` _returnvalue_x _returnvalue_y (+ _position _returnvalue_z)) false false))
    (:`Finished`
      (set `self.IsEnd` true)
      (bind _returnvalue_2 (`|CreateWidget` "/Game/Game/Widget/BPW_FonduFin.BPW_FonduFin_C"))
      (set `self.Fondu Fin` _returnvalue_2))))

(event `self.Box.OnComponentBeginOverlap`
  (params (OverlappedComponent :type "PrimitiveComponent Object Reference") (OtherActor :type "Actor Object Reference") (OtherComp :type "PrimitiveComponent Object Reference") (OtherBodyIndex :type Integer) (bFromSweep :type Boolean) (SweepResult :type "HitResult Structure (by ref)"))
  (if (`self.IsEnd`)
    (`GameplayStatics.OpenLevel` "ForestMap")))

(fn `UserConstructionScript`)