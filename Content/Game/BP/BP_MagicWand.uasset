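; BP_MagicWand is a grabbable VR wand that plays notes on musical actors it points at.
; While held, it line-traces every tick from its mesh along the Arrow's forward vector, drawing a debug line.
; Hit actors implementing BPI_Music receive PlayNoteMessage.
; The last such actor is cached and never cleared, so it only retriggers after the wand hits a different musical actor.
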(event `self.ReceiveBeginPlay`
  (bind _asvrpawn (cast `/Game/VRTemplate/Blueprints/VRPawn` (`GameplayStatics.GetPlayerPawn` 0)))
  (set `self.As VRPawn` _asvrpawn))

(event `self.ReceiveTick`
  (params (DeltaSeconds :type "Float (single-precision)"))
  (if (`/Game/VRTemplate/Blueprints/GrabComponent.bIsHeld` (`self.GrabComponent`))
    (bind (_outhit _returnvalue) (`KismetSystemLibrary.LineTraceSingle` :`Start` (`SceneComponent.K2_GetComponentLocation` (`self.StaticMesh`)) :`End` (+ (* (`SceneComponent.GetForwardVector` (`self.Arrow`)) 100000.0) (`SceneComponent.K2_GetComponentLocation` (`self.StaticMesh`))) :`TraceChannel` "TraceTypeQuery1" :`DrawDebugType` "ForOneFrame"))
    (if _returnvalue
      (bind (_bblockinghit _binitialoverlap _time _distance _location _impactpoint _normal _impactnormal _physmat _hitactor) (`GameplayStatics.BreakHitResult` _outhit))
      (if (and (`KismetSystemLibrary.DoesImplementInterface` _hitactor "/Game/Game/BP/BPI_Music.BPI_Music_C") (!= (`self.Hit Actor`) _hitactor))
        (set `self.Hit Actor` _hitactor)
        (message `/Game/Game/BP/BPI_Music.PlayNote` _hitactor)))))

(fn `UserConstructionScript`)