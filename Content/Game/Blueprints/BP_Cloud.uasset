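; Cloud actor with a configurable mesh that loops along a spline and drives the cloud material color.
; Tick places the mesh by game time, Speed and Offset, wrapped on spline length, keeping it upright and oriented along its movement.
; It also eases the shared MPC_Nuages "Alpha" toward the target or base color, following the CouleurNuages flag copied from BP_BalancoireFinal (the swing) at BeginPlay.
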(event `self.ReceiveBeginPlay`
  ;[1 1 1] Cast la balancoire pour savoir quand les nuages doivent changer de couleur
  (bind _returnvalue (`GameplayStatics.GetActorOfClass` "/Game/Game/BP/BP_BalancoireFinal.BP_BalancoireFinal_C"))
  (bind _output_get (set `self.Balancoire` _returnvalue))
  (set `self.Couleur Nuages?` (`/Game/Game/BP/BP_BalancoireFinal.CouleurNuages?` _output_get)))

(event `self.ReceiveTick`
  (params (DeltaSeconds :type "Float (single-precision)"))
  (bind _cloud (`self.Cloud`))
  (bind _returnvalue (`SplineComponent.GetLocationAtDistanceAlongSpline` (`self.Spline`) (mod (+ (* (`GameplayStatics.GetTimeSeconds`) (`self.Speed`)) (`self.Offset`)) (`SplineComponent.GetSplineLength` (`self.Spline`))) "World"))
  (`|ExecutionSequence`
    (:`then_0`
      ;[1 1 1] Suit la spline associée au nuage
      (`SceneComponent.K2_SetWorldRotation` _cloud (`KismetMathLibrary.MakeRotFromZY` (0.0 0.0 1.0) (- (`SceneComponent.K2_GetComponentLocation` _cloud) _returnvalue)) false false)
      (`SceneComponent.K2_SetWorldLocation` _cloud _returnvalue false false))
    (:`then_1`
      ;[1 1 1] Changement des couleurs du mat des nuages
      (if (`self.Couleur Nuages?`)
        (`self.GoToColor` DeltaSeconds)
        (else
          (`self.goToBaseColor` DeltaSeconds))))))

(event `GoToColor`
  (params (A :type "Float (double-precision)"))
  ;[1 1 1] Change la couleur en celle souhaitée
  (bind _returnvalue (`KismetMaterialLibrary.GetScalarParameterValue` "/Game/Game/MPC_Nuages.MPC_Nuages" "Alpha"))
  (`KismetMaterialLibrary.SetScalarParameterValue` "/Game/Game/MPC_Nuages.MPC_Nuages" "Alpha" (`KismetMathLibrary.Lerp` _returnvalue 1.0 (* A 0.5))))

(event `goToBaseColor`
  (params (A :type "Float (double-precision)"))
  ;[1 1 1] Revient a la couleur de base du mat
  (bind _returnvalue (`KismetMaterialLibrary.GetScalarParameterValue` "/Game/Game/MPC_Nuages.MPC_Nuages" "Alpha"))
  (`KismetMaterialLibrary.SetScalarParameterValue` "/Game/Game/MPC_Nuages.MPC_Nuages" "Alpha" (`KismetMathLibrary.Lerp` _returnvalue 0.0 (* A 0.5))))

(fn `UserConstructionScript`
  (`StaticMeshComponent.SetStaticMesh` (`self.Cloud`) (`self.StaticMesh`)))