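; Door whose grabbable handle moves the player from ForestMap to ZenMap2, usable only while the lighting is wide enough.
; Tick sets Active from the MPC_PostProcess Outer Radius threshold; the StartRadius read from BP_FireCamp on overlap is not used here.
; The first grab while Active plays the handle sound and drives an MPC_Fade opacity timeline, then requests the level streaming load and unload.
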(event `self.ReceiveActorBeginOverlap`
  (params (OtherActor :type "Actor Object Reference"))
  ;[1 1 1] on récupère la valeur de l'éclairage du feu dans le firecamp
  (bind _returnvalue (`GameplayStatics.GetActorOfClass` "/Game/Game/BP/BP_FireCamp.BP_FireCamp_C"))
  (set `self.Start Radius` (`/Game/Game/BP/BP_FireCamp.StartRadius` _returnvalue)))

(event `self.ReceiveTick`
  (params (DeltaSeconds :type "Float (single-precision)"))
  ;[1 1 1] Change la bool Active en fonction de l'éclairage
  (bind _returnvalue (`KismetMaterialLibrary.GetScalarParameterValue` "/Game/Game/MPC_PostProcess.MPC_PostProcess" "Outer Radius"))
  (if (>= _returnvalue 300.0)
    (set `self.Active` true)
    (else
      (set `self.Active` false))))

(event `self.GrabComponent.OnGrabbed`
  ;[1 1 1] On peut grab la poignet que si la variable Active est true
  (if (`self.Active`)
    (`/Engine/EditorBlueprintResources/StandardMacros.DoOnce` false
      (:`Completed`
        (set `self.grabbed?` true)
        ;[1 1 1] Lance le son de la porte
        (`ActorComponent.Activate` (`self.Poigneebruit`) false)
        ;[1 1 1] Fade de transition
        (bind (_direction _alpha) (`Timeline|Fade` :!via `PlayFromStart`)
          (:`Update`
            (`KismetMaterialLibrary.SetScalarParameterValue` "/Game/MPC_Fade.MPC_Fade" "Opacity" _alpha))
          (:`Finished`
            ;[1 1 1] Change de map avec le streaming level
            (`GameplayStatics.LoadStreamLevelBySoftObjectPtr` "/Game/Game/Maps/ZenMap2.ZenMap2" true)
            (`GameplayStatics.UnloadStreamLevelBySoftObjectPtr` "/Game/Game/Maps/ForestMap.ForestMap")))))))

(fn `UserConstructionScript`)