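; BP_FireCamp is a campfire that grows its lit area when a branch's cylinder enters its sphere.
; It activates the branch's fire particles, then a timeline widens the radii in MPC_PostProcess.
; The branch is flagged destroyed; non-firefly branches are also force-released from the player and get their grab type changed.
; Tick sets ActiveFlarDoor once the stored start radius is large enough, meant to send Flar toward the door.
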(event `self.Sphere.OnComponentBeginOverlap`
  (params (OverlappedComponent :type "PrimitiveComponent Object Reference") (OtherActor :type "Actor Object Reference") (OtherComp :type "PrimitiveComponent Object Reference") (OtherBodyIndex :type Integer) (bFromSweep :type Boolean) (SweepResult :type "HitResult Structure (by ref)"))
  (bind _asbp_branche (cast `/Game/Game/BP/BP_Branche` OtherActor))
  (if (== OtherComp (`/Game/Game/BP/BP_Branche.Cylinder` _asbp_branche))
    (`|ExecutionSequence`
      (:`then_0`
        ;[1 1 1] 1:Active les particules
        (`ActorComponent.Activate` (`/Game/Game/BP/BP_Branche.FeuFeuFeu` _asbp_branche) false))
      (:`then_1`
        ;[1 1 1] Augmente la taille de l'éclairage du feu
        (bind _returnvalue (`KismetMaterialLibrary.GetScalarParameterValue` "/Game/Game/MPC_PostProcess.MPC_PostProcess" "Outer Radius"))
        (set `self.StartRadius` _returnvalue)
        (`KismetMaterialLibrary.SetScalarParameterValue` "/Game/Game/MPC_PostProcess.MPC_PostProcess" "Time" (`GameplayStatics.GetTimeSeconds`))
        (bind (_direction _alpha) (`Timeline|Timeline` :!via `PlayFromStart`)
          (:`Update`
            (bind _returnvalue_2 (`KismetMathLibrary.Lerp` (`self.StartRadius`) (+ (`self.StartRadius`) 150.0) _alpha))
            (`KismetMaterialLibrary.SetScalarParameterValue` "/Game/Game/MPC_PostProcess.MPC_PostProcess" "Outer Radius" _returnvalue_2)
            (`KismetMaterialLibrary.SetScalarParameterValue` "/Game/Game/MPC_PostProcess.MPC_PostProcess" "Inner Radius" (- _returnvalue_2 50.0))
            ;[1 1 1] Détruit la branche
            (bind _asbp_branche_luciole (cast `/Game/Game/BP/BP_BrancheLuciole` OtherActor)
              (:`then`
                (`/Engine/EditorBlueprintResources/StandardMacros.IsValid` _asbp_branche_luciole
                  (:`Is Valid`
                    (set `/Game/Game/BP/BP_Branche.IsDestroyed` true _asbp_branche_luciole))))
              (:`CastFailed`
                ;[1 1 1] Force le joueur a lacher la branche
                (set `/Game/Game/BP/BP_Branche.IsDestroyed` true _asbp_branche)
                (bind _grabcomponent (`/Game/Game/BP/BP_Branche.GrabComponent` _asbp_branche))
                (`/Game/VRTemplate/Blueprints/GrabComponent.TryRelease` _grabcomponent)
                (set `/Game/VRTemplate/Blueprints/GrabComponent.GrabType` "NewEnumerator0" _grabcomponent)))))))))

(event `self.ReceiveTick`
  (params (DeltaSeconds :type "Float (single-precision)"))
  ;[1 1 1] Quand le feu est assez grand, on lance un evenement qui va faire en sorte que flar va vers la porte
  (if (>= (`self.StartRadius`) 900.0)
    (set `self.ActiveFlarDoor` true)))

(fn `UserConstructionScript`)