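; BP_Flar is a grabbable VR companion that hovers, bobbing, in front of the player's camera.
; Five seconds after BeginPlay, timelines blend it onto a spline cinematic and back; it can carry the BP_BrancheLuciole branch.
; A Gate detects release, fading throw velocity while ramping follow strength.
; Each release also advances a color counter, reset after ten idle seconds, with the color eased into MPC_Flar.
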(event `self.ReceiveBeginPlay`
  (`|ExecutionSequence`
    (:`then_0`
      (bind _asvrpawn (cast `/Game/VRTemplate/Blueprints/VRPawn` (`GameplayStatics.GetPlayerPawn` 0)))
      (set `self.As VRPawn` _asvrpawn))
    (:`then_1`
      (bind _returnvalue (`GameplayStatics.GetActorOfClass` "/Game/Game/BP/BP_BrancheLuciole.BP_BrancheLuciole_C"))
      (set `self.brancheluciole` _returnvalue))
    (:`then_2`
      (`KismetSystemLibrary.Delay` 5.0)
      (`self.MoveFlar`))))

(event `MoveFlar`
  (`|ExecutionSequence`
    (:`then_0`
      (bind (_direction _newtrack_0) (`Timeline|MoveFlarT` :!via `PlayFromStart`)
        (:`Update`
          (bind _splineref (`self.SplineREF`)
            (:`then`
              (bind _spline (`/Game/Game/BP/BP_SplineLuciole.Spline` _splineref))
              (set `self.SplineLocation` (`SplineComponent.GetLocationAtDistanceAlongSpline` _spline (`KismetMathLibrary.Lerp` 0.0 (`SplineComponent.GetSplineLength` _spline) _newtrack_0) "World")))
            (:`else`)))
        (:`Finished`
          (set `/Game/Game/BP/BP_BrancheLuciole.followflar` false (`self.brancheluciole`))
          (bind (_direction_2 _alpha) (`Timeline|AlphaCinematique` :!via `Reverse` :!label _label)
            (:`Update`
              (set `self.AlphaCine` _alpha))))))
    (:`then_1`
      (goto _label))))

(event `self.ReceiveTick`
  (params (DeltaSeconds :type "Float (single-precision)"))
  (bind (_returnvalue_x _returnvalue_y _returnvalue_z) (`KismetMathLibrary.BreakVector` (`self.K2_GetActorLocation`)))
  (`|ExecutionSequence`
    (:`then_0`
      (`self.KeepInCamera` DeltaSeconds)
      (if (`self.FlarGrabBranch?`)
        (`self.K2_SetActorLocation` (`self.brancheluciole`) (`KismetMathLibrary.MakeVector` _returnvalue_x _returnvalue_y (- _returnvalue_z (`self.bone`))) false false)))
    (:`then_1`
      (if (`/Game/VRTemplate/Blueprints/GrabComponent.bIsHeld` (`self.GrabComponent`))
        (goto _label_2 :!via `Open`)
        (else
          (`/Engine/EditorBlueprintResources/StandardMacros.Gate` true :!label _label_2
            (:`Exit`
              (`|ExecutionSequence`
                (:`then_0`
                  (`KismetSystemLibrary.Delay` 1.0)
                  (set `self.Compteur` (+ (`self.Compteur`) 1))
                  (switch `int` (`self.Compteur`)
                    (:`0`
                      (set `self.TargetColor` (`KismetMathLibrary.Conv_ColorToLinearColor` (`KismetMathLibrary.Conv_LinearColorToColor` (struct :`R` 1.0 :`G` 1.0 :`B` 1.0 :`A` 1.0)))))
                    (:`1`
                      (set `self.TargetColor` (`KismetMathLibrary.Conv_ColorToLinearColor` (`KismetMathLibrary.Conv_LinearColorToColor` (struct :`R` 1.0 :`G` 0.916666 :`A` 1.0)))))
                    (:`2`
                      (set `self.TargetColor` (`KismetMathLibrary.Conv_ColorToLinearColor` (`KismetMathLibrary.Conv_LinearColorToColor` (struct :`G` 0.01411 :`B` 1.0 :`A` 1.0)))))
                    (:`3`
                      (set `self.TargetColor` (`KismetMathLibrary.Conv_ColorToLinearColor` (`KismetMathLibrary.Conv_LinearColorToColor` (struct :`R` 1.0 :`B` 0.007289 :`A` 1.0)))))
                    (:`4`
                      (set `self.TargetColor` (`KismetMathLibrary.Conv_ColorToLinearColor` (`KismetMathLibrary.Conv_LinearColorToColor` (struct :`G` 1.0 :`A` 1.0)))))
                    (:`5`
                      (set `self.TargetColor` (`KismetMathLibrary.Conv_ColorToLinearColor` (`KismetMathLibrary.Conv_LinearColorToColor` (struct :`R` 0.322 :`B` 1.0 :`A` 1.0))))))
                  (`KismetSystemLibrary.RetriggerableDelay` 10.0)
                  (set `self.Compteur` 0)
                  (set `self.TargetColor` (`KismetMathLibrary.Conv_ColorToLinearColor` (`KismetMathLibrary.Conv_LinearColorToColor` (struct :`R` 1.0 :`G` 1.0 :`B` 1.0 :`A` 1.0)))))
                (:`then_1`
                  (bind (_direction _alpha) (`Timeline|Timeline` :!via `PlayFromStart`)
                    (:`Update`
                      (`PrimitiveComponent.SetPhysicsLinearVelocity` (`self.Sphere`) (`KismetMathLibrary.VLerp` (`/Game/VRTemplate/Blueprints/GrabComponent.AverageVelocity` (`self.GrabComponent`)) (0.0 0.0 0.0) _alpha) false "None")
                      (set `self.Alpha` (* _alpha 3.5)))))
                (:`then_2`
                  (goto _label_2 :!via `Close`))))))))
    (:`then_2`
      (bind _returnvalue (`KismetMaterialLibrary.GetVectorParameterValue` "/Game/Game/Flar/MPC_Flar.MPC_Flar" "Color"))
      (`KismetMaterialLibrary.SetVectorParameterValue` "/Game/Game/Flar/MPC_Flar.MPC_Flar" "Color" (`KismetMathLibrary.LinearColorLerp` _returnvalue (`self.TargetColor`) (* DeltaSeconds 2.5))))))

(fn `KeepInCamera`
  (params (`Delta Seconds` :type "Float (double-precision)"))
  (bind _camera (`/Game/VRTemplate/Blueprints/VRPawn.Camera` (`self.As VRPawn`)))
  (if (not (`/Game/VRTemplate/Blueprints/GrabComponent.bIsHeld` (`self.GrabComponent`)))
    (`self.K2_SetActorLocation` (`KismetMathLibrary.VLerp` (`KismetMathLibrary.VLerp` (`self.K2_GetActorLocation`) (+ (+ (+ (`SceneComponent.K2_GetComponentLocation` _camera) (* (`SceneComponent.GetForwardVector` _camera) (50.0 50.0 0.0))) (* (`SceneComponent.GetRightVector` _camera) 20.0)) (`KismetMathLibrary.MakeVector` 0.0 0.0 (* (`KismetMathLibrary.Sin` (* (`GameplayStatics.GetTimeSeconds`) 3.0)) 4.0))) (* `Delta Seconds` (`self.Alpha`))) (`self.SplineLocation`) (`self.AlphaCine`)) false true)))

(fn `UserConstructionScript`)